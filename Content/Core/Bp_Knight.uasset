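; Knight pawn with hand-written platformer movement along Y and Z, using Grounded, Jumping, Rising and Falling modes.
; Input, per-mode gravity and timed jump thrust feed AddedVelocity; releasing jump early cuts the rise.
; Each tick applies clamped velocity through swept moves, slides along blocking hits, then derives velocity from actual displacement.
; Floor-like capsule hits set Grounded and restart a near-zero timer that reverts to Falling once contact stops.
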(event OnComponentHit(Capsule)
  (params (HitComponent :type Primitive%20Component%20Object%20Reference) (OtherActor :type Actor%20Object%20Reference) (OtherComp :type Primitive%20Component%20Object%20Reference) (NormalImpulse :type Vector :default "0, 0, 0") (Hit :type Hit%20Result%20Structure%20%28by%20ref%29))
  (if (>= (Math|Vector|DotProduct (.normal Hit) "0, 0,1.000000") 0.71)
    (Variables|Default|SetHeight (.z (Transformation|GetActorLocation)))
    (Movement|ChangeMovement "NewEnumerator0")
    (Utilities|Time|SetTimerbyFunctionName self "Ungrounded" 1e-06)))

(event EventBeginPlay
  (Utilities|FlowControl|Delay 0.5)
  (Jump|StartJump))

(event EventTick
  (params (DeltaSeconds :type Float%20%28single-precision%29))
  (Utilities|FlowControl|Sequence
    (:then_0
      (Gravity|Gravity)
      (Jump|Jumping))
    (:then_1
      (Movement|ResolveMovement))))

(event Input|ActionEvents|InputActionJump
  (params (Key :type Key%20Structure))
  (:Pressed
    (Jump|StartJump))
  (:Released
    (Jump|StopJump true)))

(event Input|AxisEvents|InputAxisRight
  (params (AxisValue :type Float%20%28single-precision%29))
  (Movement|AddVelocity "0.000000,1.000000,0.000000" (* (Math|Float|Sign(Float) AxisValue) (Variables|Movement|GetMoveRightAccel))))

(fn ConstructionScript)

(fn AddVelocity
  (params (Direcion :type Vector) (Scale :type Float%20%28single-precision%29))
  (Variables|Movement|SetAddedVelocity (+ (* Direcion (* Scale (Utilities|Time|GetWorldDeltaSeconds))) (Variables|Movement|GetAddedVelocity))))

(fn ResolveMovement
  (bind _maxwalkspeed (Variables|Movement|GetMaxWalkSpeed))
  (bind _movementmode (Variables|Movement|GetMovementMode))
  (bind _maxfallspeed (Variables|Gravity|GetMaxFallSpeed))
  (LocalVariables|SetLocationBefore (Transformation|GetActorLocation))
  (Utilities|FlowControl|Sequence
    (:then_0
      (bind _sweephitresult (Transformation|SetActorLocation (+ (Transformation|GetActorLocation) (* (Math|Vector|MakeVector (.X (Math|Vector|BreakVector (+ (Variables|Movement|GetVelocity) (Variables|Movement|GetAddedVelocity)))) (Math|Float|Clamp(Float) (|InstantAccel (.Y (Math|Vector|BreakVector (+ (Variables|Movement|GetVelocity) (Variables|Movement|GetAddedVelocity))))) (* _maxwalkspeed -1.0) _maxwalkspeed) (Math|Float|Clamp(Float) (.Z (Math|Vector|BreakVector (+ (Variables|Movement|GetVelocity) (Variables|Movement|GetAddedVelocity)))) (Utilities|Select :Index (Variables|Movement|GetMovementMode) :NewEnumerator0 _maxfallspeed :NewEnumerator1 0.0 :NewEnumerator3 0.0 :NewEnumerator2 _maxfallspeed) (Variables|Jump|GetJumpSpeedCap))) (Utilities|Time|GetWorldDeltaSeconds))) true false))
      (bind _output_get (LocalVariables|SetLocalSweep _sweephitresult))
      (while (.bBlockingHit (Collision|BreakHitResult _output_get))
        (bind _sweephitresult_2 (Transformation|SetActorLocation (+ (Transformation|GetActorLocation) (- (- (.TraceEnd (Collision|BreakHitResult _output_get)) (.TraceStart (Collision|BreakHitResult _output_get))) (* (.ImpactNormal (Collision|BreakHitResult _output_get)) (Math|Vector|DotProduct (.ImpactNormal (Collision|BreakHitResult _output_get)) (- (.TraceEnd (Collision|BreakHitResult _output_get)) (.TraceStart (Collision|BreakHitResult _output_get))))))) true false))
        (LocalVariables|SetLocalSweep _sweephitresult_2)))
    (:then_1
      (Utilities|FlowControl|Sequence
        (:then_0
          (Variables|Movement|SetVelocity (/ (- (Transformation|GetActorLocation) (LocalVariables|GetLocationBefore)) (Utilities|Time|GetWorldDeltaSeconds)))
          (Variables|Movement|SetAddedVelocity "0, 0, 0"))
        (:then_1
          (if (or (Utilities|Enum|Equal(Enum) _movementmode "NewEnumerator1") (Utilities|Enum|Equal(Enum) _movementmode "NewEnumerator3"))
            (if (<= (.z (Variables|Movement|GetVelocity)) 0.0)
              (Movement|ChangeMovement "NewEnumerator2"))))))))

(fn ChangeMovement
  (params (NewMovement :type EMovement%20Enum :default "NewEnumerator0"))
  (LocalVariables|SetOldMovement (Variables|Movement|GetMovementMode))
  (switch Utilities|FlowControl|Switch|SwitchonEMovement NewMovement
    (:NewEnumerator0
      (Variables|Movement|SetMovementMode NewMovement :!label _label)
      (return (Utilities|Enum|NotEqual(Enum) (LocalVariables|GetOldMovement) NewMovement)))
    (:NewEnumerator1
      (goto _label))
    (:NewEnumerator3
      (goto _label))
    (:NewEnumerator2
      (if (Utilities|Enum|NotEqual(Enum) (Variables|Movement|GetMovementMode) "NewEnumerator1")
        (goto _label)))))

(fn Gravity
  (bind _gravityacceleration (Variables|Gravity|GetGravityAcceleration))
  (Movement|AddVelocity "0, 0,-1.000000" (Utilities|Select :Index (Variables|Movement|GetMovementMode) :NewEnumerator0 _gravityacceleration :NewEnumerator1 0.0 :NewEnumerator3 (Variables|Gravity|GetRisingGravityAcceleration) :NewEnumerator2 _gravityacceleration)))

(fn StartJump
  (if (Utilities|Enum|Equal(Enum) (Variables|Movement|GetMovementMode) "NewEnumerator0")
    (Variables|Jump|SetJumpTimer 0.0)
    (Movement|ChangeMovement "NewEnumerator1")))

(fn Jumping
  (if (Utilities|Enum|Equal(Enum) (Variables|Movement|GetMovementMode) "NewEnumerator1")
    (Movement|AddVelocity "0, 0,1.000000" (Variables|Jump|GetJumpAcceleration))
    (bind _output_get (Variables|Jump|SetJumpTimer (+ (Variables|Jump|GetJumpTimer) (Utilities|Time|GetWorldDeltaSeconds))))
    (if (>= _output_get (Variables|Jump|GetJumpMaxDuration))
      (Jump|StopJump false))))

(fn StopJump
  (params (bSharp :type Boolean))
  (if (Utilities|Enum|Equal(Enum) (Variables|Movement|GetMovementMode) "NewEnumerator1")
    (Movement|ChangeMovement "NewEnumerator3")
    (if bSharp
      (Movement|AddVelocity "0, 0,-1.000000" (Math|Float|Absolute(Float) (/ (/ (.z (Variables|Movement|GetVelocity)) (Utilities|Time|GetWorldDeltaSeconds)) 1.5))))))

(fn Ungrounded
  (if (not (CallFunction|InAir))
    (Movement|ChangeMovement "NewEnumerator2")))

(fn InAir
  (bind _movementmode (Variables|Movement|GetMovementMode))
  (return (Math|Boolean|ORBoolean (Utilities|Enum|Equal(Enum) _movementmode "NewEnumerator1") (Utilities|Enum|Equal(Enum) _movementmode "NewEnumerator2") (Utilities|Enum|Equal(Enum) _movementmode "NewEnumerator3"))))